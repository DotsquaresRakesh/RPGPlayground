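; Base character Blueprint using the Gameplay Ability System for sword melee combat and death.
; It acquires GA_Melee on BeginPlay and activates it by class on MeleeAttack.
; SwordCollider overlaps with hostile characters send a Skills.Melee.DealDamage gameplay event to itself with the victim as target, leaving damage to event listeners.
; Die plays the Shinbi death montage, waits out its length, then destroys the actor.
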(event `self.ReceiveBeginPlay`
  (`self.AcquireAbility` "/Game/Blueprints/Characters/GameplayAbilities/Melee/GA_Melee.GA_Melee_C"))

(event `self.ReceiveTick`
  (params (DeltaSeconds :type "Float (single-precision)")))

(event `self.BP_Die`
  (bind _returnvalue (`self.PlayAnimMontage` "/Game/Blueprints/Characters/Animation/AM_Shinbi_Die.AM_Shinbi_Die"))
  (`KismetSystemLibrary.Delay` _returnvalue)
  (`self.K2_DestroyActor`))

(event `MeleeAttack`
  ;[1 1 1] Melee
  (`AbilitySystemComponent.TryActivateAbilityByClass` (`self.AbilitySystemComp`) "/Game/Blueprints/Characters/GameplayAbilities/Melee/GA_Melee.GA_Melee_C" true))

(event `self.SwordCollider.OnComponentBeginOverlap`
  (params (OverlappedComponent :type "PrimitiveComponent Object Reference") (OtherActor :type "Actor Object Reference") (OtherComp :type "PrimitiveComponent Object Reference") (OtherBodyIndex :type Integer) (bFromSweep :type Boolean) (SweepResult :type "HitResult Structure (by ref)"))
  ;[1 1 1] Sword Overlap Event
  (if (!= OtherActor self)
    (bind _ascharacter_base (cast `CharacterBase` OtherActor))
    (bind _returnvalue (`self.IsOtherHostile` _ascharacter_base self))
    (if _returnvalue
      (`AbilitySystemBlueprintLibrary.SendGameplayEventToActor` self (struct :`TagName` "Skills.Melee.DealDamage") (make `GameplayEventData` (struct) null OtherActor)))))

(fn `UserConstructionScript`)