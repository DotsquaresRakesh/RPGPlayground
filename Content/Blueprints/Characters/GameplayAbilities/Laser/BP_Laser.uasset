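; Laser beam actor for the laser gameplay ability, tracking hostile characters at the beam's end and requesting damage on them.
; LaserEndDetector overlaps add characters hostile to the instigator to a list and remove them on exit.
; A looping timer sends that list to the instigator as target data in a Skills.Laser.DealDamage gameplay event.
; Tick stretches the mesh to the detector by setting the anim instance's end-bone offset.
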(event `self.ReceiveBeginPlay`
  (set `self.LaserBeamLength` (`KismetMathLibrary.VSize` (- (`SceneComponent.GetSocketLocation` (`self.LaserMesh`) "end") (`self.K2_GetActorLocation`))))
  ;[1 1 1] SendDamageEvent
  (`KismetSystemLibrary.K2_SetTimerDelegate` (delegate `SendDealDamageEvent`) 0.3 true))

(event `SendDealDamageEvent`
  ;[1 1 1] SendDamageEvent
  (if (`KismetMathLibrary.Conv_IntToBool` (`KismetArrayLibrary.Array_Length` (`self.OverlappingActors`)))
    _
    (else
      _))
  (`AbilitySystemBlueprintLibrary.SendGameplayEventToActor` (`self.GetInstigator`) (struct :`TagName` "Skills.Laser.DealDamage") (make `GameplayEventData` (struct) null null null null (struct) (struct) (struct) 0.0 (`AbilitySystemBlueprintLibrary.AbilityTargetDataFromActorArray` (`self.OverlappingActors`)))))

(event `self.ReceiveTick`
  (params (DeltaSeconds :type "Float (single-precision)"))
  (bind _asabp_laser_beam (cast `/Game/Blueprints/Characters/GameplayAbilities/Laser/LaserAssets/ABP_LaserBeam` (`SkeletalMeshComponent.GetAnimInstance` (`self.LaserMesh`))))
  (set `/Game/Blueprints/Characters/GameplayAbilities/Laser/LaserAssets/ABP_LaserBeam.EndBoneOffset` (`KismetMathLibrary.MakeVector` (- (`KismetMathLibrary.VSize` (- (`self.K2_GetActorLocation`) (`SceneComponent.K2_GetComponentLocation` (`self.LaserEndDetector`)))) (`self.LaserBeamLength`))) _asabp_laser_beam))

(event `self.LaserEndDetector.OnComponentBeginOverlap`
  (params (OverlappedComponent :type "PrimitiveComponent Object Reference") (OtherActor :type "Actor Object Reference") (OtherComp :type "PrimitiveComponent Object Reference") (OtherBodyIndex :type Integer) (bFromSweep :type Boolean) (SweepResult :type "HitResult Structure (by ref)"))
  (bind _asbp_character_base (cast `/Game/Blueprints/Characters/BP_CharacterBase` OtherActor))
  (bind _asbp_character_base_2 (cast `/Game/Blueprints/Characters/BP_CharacterBase` (`self.GetInstigator`)))
  (bind _returnvalue (`CharacterBase.IsOtherHostile` _asbp_character_base_2 _asbp_character_base))
  (if _returnvalue
    (`KismetArrayLibrary.Array_AddUnique` (`self.OverlappingActors`) _asbp_character_base)))

(event `self.LaserEndDetector.OnComponentEndOverlap`
  (params (OverlappedComponent :type "PrimitiveComponent Object Reference") (OtherActor :type "Actor Object Reference") (OtherComp :type "PrimitiveComponent Object Reference") (OtherBodyIndex :type Integer))
  (bind _asbp_character_base (cast `/Game/Blueprints/Characters/BP_CharacterBase` OtherActor))
  (`KismetArrayLibrary.Array_RemoveItem` (`self.OverlappingActors`) _asbp_character_base))

(fn `UserConstructionScript`)